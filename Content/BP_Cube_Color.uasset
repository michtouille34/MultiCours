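; BP_Cube_Color is a cube actor that takes a random color and gets launched when its Color event fires.
; The event randomizes VectorColor and applies the scaled Impulse argument to the Cube as a velocity-change impulse, ignoring mass.
; VectorColor uses RepNotify, so its OnRep function writes the value to the "Base Color" material parameter, keeping the color in sync across the network.
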(event Custom|Color
  (params (Impulse :type Vector))
  (Variables|Default|SetVectorColor (Math|Vector|MakeVector (Math|Random|RandomFloat) (Math|Random|RandomFloat) (Math|Random|RandomFloat)))
  (Physics|AddImpulse (Variables|Default|GetCube) (* Impulse 1e+03) "None" true))

(event EventBeginPlay)

(event Collision|EventActorBeginOverlap
  (params (OtherActor :type Actor%20Object%20Reference)))

(event EventTick
  (params (DeltaSeconds :type Float%20%28single-precision%29)))

(fn ConstructionScript)

(fn OnRepVectorColor
  (Rendering|Material|SetVectorParameterValueonMaterials (Variables|Default|GetCube) "Base Color" (Variables|Default|GetVectorColor)))